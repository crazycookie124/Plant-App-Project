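; BP_CameraManager switches the player's view between fixed hallway, kitchen and living room cameras, starting in the hallway.
; Each room switch event changes the view target, adds a newly created HUD widget for that room without removing earlier ones, and records the room number.
; A day/night button event advances a wrapping three-state day counter through FindNum and stores the result in GlobalDayNum.
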(event `self.ReceiveBeginPlay`
  (`PlayerController.SetViewTargetWithBlend` (`GameplayStatics.GetPlayerController` 0) (`self.HallWayCamera`) 0.0 "VTBlend_Linear" 0.0 false))

(event `/Game/CommunityPlant/Core/BluePrints/BPI_CameraManager.KSwitchCam`
  (`PlayerController.SetViewTargetWithBlend` (`GameplayStatics.GetPlayerController` 0) (`self.KitchenCamera`) 0.0 "VTBlend_Linear" 0.0 false)
  (bind _returnvalue (`|CreateWidget` "/Game/CommunityPlant/Core/UserInterface/WBP_K_HUD.WBP_K_HUD_C"))
  (`UserWidget.AddToViewport` _returnvalue 0)
  (set `self.Room Num` 1))

(event `/Game/CommunityPlant/Core/BluePrints/BPI_CameraManager.HSwitchCam`
  (`PlayerController.SetViewTargetWithBlend` (`GameplayStatics.GetPlayerController` 0) (`self.HallWayCamera`) 0.0 "VTBlend_Linear" 0.0 false)
  (bind _returnvalue (`|CreateWidget` "/Game/CommunityPlant/Core/UserInterface/WBP_H_HUD.WBP_H_HUD_C"))
  (`UserWidget.AddToViewport` _returnvalue 0)
  (set `self.Room Num` 0))

(event `/Game/CommunityPlant/Core/BluePrints/BPI_CameraManager.LSwitchCam`
  (`PlayerController.SetViewTargetWithBlend` (`GameplayStatics.GetPlayerController` 0) (`self.LivingRoomCamera`) 0.0 "VTBlend_Linear" 0.0 false)
  (bind _returnvalue (`|CreateWidget` "/Game/CommunityPlant/Core/UserInterface/WBP_L_HUD.WBP_L_HUD_C"))
  (`UserWidget.AddToViewport` _returnvalue 0)
  (set `self.Room Num` 2))

(event `/Game/CommunityPlant/Core/BluePrints/BPI_CameraManager.DayNightBPressed`
  (bind _dayout (`self.FindNum`))
  (set `self.GlobalDayNum` _dayout))

(fn `FindNum`
  (returns (DayOut :type Integer))
  (bind _daynum (`self.DayNum`))
  (if (< _daynum 2)
    (bind _result (`/Engine/EditorBlueprintResources/StandardMacros.IncrementInt` _daynum)
      (:`  `
        (return _result)))
    (else
      (bind _output_get (set `self.DayNum` 0))
      (return _output_get))))

(fn `UserConstructionScript`)