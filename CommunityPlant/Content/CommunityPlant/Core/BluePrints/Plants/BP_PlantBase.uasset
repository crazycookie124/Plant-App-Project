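; Base plant actor that shows a 2D sprite for its plant type and can be dragged by touch when flagged moveable.
; On BeginPlay it caches the BP_DeafultSpawnn actor, enables input, and sets its sprite from the PlantDataTable row matching PlantType.
; While dragging, Tick deprojects the first touch to world X and Z, locking Y to the spawn actor's root so the plant stays on one plane.
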(event `self.ReceiveBeginPlay`
  (bind _plantdatatable (`self.PlantDataTable`))
  (bind _planttype (`self.PlantType`))
  (bind _returnvalue (`GameplayStatics.GetActorOfClass` "/Game/CommunityPlant/Core/BluePrints/Plants/BP_DeafultSpawnn.BP_DeafultSpawnn_C"))
  (set `self.SpawnRef` _returnvalue)
  (`self.EnableInput` null)
  (if (not (`self.PlantTypeCast`))
    (`KismetSystemLibrary.Delay` 0.1))
  (bind _outrownames (`DataTableFunctionLibrary.GetDataTableRowNames` _plantdatatable))
  (for _array_element _outrownames
    (if (== _array_element _planttype)
      (bind _returnvalue_2 (`|GetDataTableRow` _plantdatatable _planttype)
        (:`then`
          (`PaperSpriteComponent.SetSprite` (`self.PlantSprite`) (`.Image_11_0919C0B5418850D2360BB1AE92C7B97D` (break `/Game/CommunityPlant/Core/BluePrints/Plants/S_PlantData` _returnvalue_2))))))))

(event `self.ReceiveActorOnInputTouchBegin`
  (params (FingerIndex :type "ETouchIndex Enum" :default "Touch1"))
  (if (`self.PlantMoveable?`)
    (set `self.IsDragging?` true)))

(event `self.ReceiveActorOnInputTouchEnd`
  (params (FingerIndex :type "ETouchIndex Enum" :default "Touch1"))
  (set `self.IsDragging?` false))

(event `self.ReceiveTick`
  (params (DeltaSeconds :type "Float (single-precision)"))
  (bind _returnvalue (`GameplayStatics.GetPlayerController` 0))
  (bind (_locationx _locationy) (`PlayerController.GetInputTouchState` _returnvalue "Touch1"))
  (bind _worldposition (`GameplayStatics.DeprojectScreenToWorld` _returnvalue (`KismetMathLibrary.MakeVector2D` _locationx _locationy)))
  (if (`self.IsDragging?`)
    (`self.K2_SetActorLocation` (`KismetMathLibrary.MakeVector` (.x _worldposition) (.y (.location (`SceneComponent.K2_GetComponentToWorld` (`/Game/CommunityPlant/Core/BluePrints/Plants/BP_DeafultSpawnn.DefaultSceneRoot` (`self.SpawnRef`))))) (.z _worldposition)))))

(fn `UserConstructionScript`)