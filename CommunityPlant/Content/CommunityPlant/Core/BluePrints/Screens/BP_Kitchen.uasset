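; BP_Kitchen is a kitchen screen that switches its tile map visuals between day, sunset and night.
; The Day/nightPressed event calls FindNum, which advances a stored counter and wraps it to zero to cycle the three states.
; Each state sets a matching tile map on the RenderComponent and swaps material slot 0 to that time's overlay blend material instance.
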(event `/Game/CommunityPlant/Core/BluePrints/BPI_CameraManager.Day/nightPressed`
  (bind _rendercomponent (`self.RenderComponent`))
  (bind _dayout (`self.FindNum`))
  (switch `int` _dayout
    (:`0`
      (`PaperTileMapComponent.SetTileMap` _rendercomponent "/Game/CommunityPlant/Assets/HouseAssets/TileMaps/KitchenTileMaps/DKitchenExport_TileMap.DKitchenExport_TileMap")
      (`PrimitiveComponent.SetMaterial` _rendercomponent 0 "/Game/CommunityPlant/Assets/HouseAssets/Materials/Kitchen_Materials/M_K_DayOverlayBlend_Inst.M_K_DayOverlayBlend_Inst"))
    (:`1`
      (`PaperTileMapComponent.SetTileMap` _rendercomponent "/Game/CommunityPlant/Assets/HouseAssets/TileMaps/KitchenTileMaps/SKitchenExport_TileMap.SKitchenExport_TileMap")
      (`PrimitiveComponent.SetMaterial` _rendercomponent 0 "/Game/CommunityPlant/Assets/HouseAssets/Materials/Kitchen_Materials/M_K_SunSetOverlayBlend_Inst.M_K_SunSetOverlayBlend_Inst"))
    (:`2`
      (`PaperTileMapComponent.SetTileMap` _rendercomponent "/Game/CommunityPlant/Assets/HouseAssets/TileMaps/KitchenTileMaps/NKitchenExport_TileMap.NKitchenExport_TileMap")
      (`PrimitiveComponent.SetMaterial` _rendercomponent 0 "/Game/CommunityPlant/Assets/HouseAssets/Materials/Kitchen_Materials/M_K_NightOverlayBlend_Inst.M_K_NightOverlayBlend_Inst"))))

(fn `FindNum`
  (returns (DayOut :type Integer))
  (locals (DayNum :type Integer))
  (bind _num (`self.Num`))
  (if (< _num 2)
    (bind _result (`/Engine/EditorBlueprintResources/StandardMacros.IncrementInt` _num)
      (:`  `
        (return _result)))
    (else
      (bind _output_get (set `self.Num` 0))
      (return _output_get))))

(fn `UserConstructionScript`)