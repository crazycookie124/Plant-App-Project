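; Living room screen tile map actor that switches between day, sunset and night looks.
; Each Day/nightPressed event calls FindNum, which cycles a counter through three states and wraps back to zero.
; The resulting index selects both the tile map asset and its matching overlay blend material instance on the render component.
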(event `/Game/CommunityPlant/Core/BluePrints/BPI_CameraManager.Day/nightPressed`
  (bind _rendercomponent (`self.RenderComponent`))
  (bind _dayout (`self.FindNum`))
  (switch `int` _dayout
    (:`0`
      (`PaperTileMapComponent.SetTileMap` _rendercomponent "/Game/CommunityPlant/Assets/HouseAssets/TileMaps/LivingRoomTileMaps/DLivingRoomExport_TileMap.DLivingRoomExport_TileMap")
      (`PrimitiveComponent.SetMaterial` _rendercomponent 0 "/Game/CommunityPlant/Assets/HouseAssets/Materials/LivingRoomMaterials/M_L_DayOverlayBlend_Inst.M_L_DayOverlayBlend_Inst"))
    (:`1`
      (`PaperTileMapComponent.SetTileMap` _rendercomponent "/Game/CommunityPlant/Assets/HouseAssets/TileMaps/LivingRoomTileMaps/SLivingRoomExport_TileMap.SLivingRoomExport_TileMap")
      (`PrimitiveComponent.SetMaterial` _rendercomponent 0 "/Game/CommunityPlant/Assets/HouseAssets/Materials/LivingRoomMaterials/M_L_SunSetOverlayBlend_Inst.M_L_SunSetOverlayBlend_Inst"))
    (:`2`
      (`PaperTileMapComponent.SetTileMap` _rendercomponent "/Game/CommunityPlant/Assets/HouseAssets/TileMaps/LivingRoomTileMaps/NLivingRoomExport_TileMap.NLivingRoomExport_TileMap")
      (`PrimitiveComponent.SetMaterial` _rendercomponent 0 "/Game/CommunityPlant/Assets/HouseAssets/Materials/LivingRoomMaterials/M_L_NightOverlayBlend_Inst.M_L_NightOverlayBlend_Inst"))))

(fn `FindNum`
  (returns (DayOut :type Integer))
  (locals (DayNum :type Integer))
  (bind _num (`self.Num`))
  (if (< _num 2)
    (bind _result (`/Engine/EditorBlueprintResources/StandardMacros.IncrementInt` _num)
      (:`  `
        (return _result)))
    (else
      (bind _output_get (set `self.Num` 0))
      (return _output_get))))

(fn `UserConstructionScript`)