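; BP_Hallway is a hallway screen actor that switches its tile map look between day, sunset and night.
; Each Day/nightPressed event calls FindNum, which advances DayNum and wraps it to zero after two.
; The result selects the tile map for the render component and its matching overlay blend material.
; BeginPlay, Tick and the construction script contain no logic.
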(event `self.ReceiveBeginPlay`)

(event `/Game/CommunityPlant/Core/BluePrints/BPI_CameraManager.Day/nightPressed`
  (bind _rendercomponent (`self.RenderComponent`))
  (bind _dayout (`self.FindNum`))
  (switch `int` _dayout
    (:`0`
      (`PaperTileMapComponent.SetTileMap` _rendercomponent "/Game/CommunityPlant/Assets/HouseAssets/TileMaps/HallwayTilemaps/D_HallwaySpriteSheet_TileMap.D_HallwaySpriteSheet_TileMap")
      (`PrimitiveComponent.SetMaterial` _rendercomponent 0 "/Game/CommunityPlant/Assets/HouseAssets/Materials/Hallway_Materials/M_H_DayOverlayBlend_Inst.M_H_DayOverlayBlend_Inst"))
    (:`1`
      (`PaperTileMapComponent.SetTileMap` _rendercomponent "/Game/CommunityPlant/Assets/HouseAssets/TileMaps/HallwayTilemaps/S_HallwaySpriteSheet_TileMap.S_HallwaySpriteSheet_TileMap")
      (`PrimitiveComponent.SetMaterial` _rendercomponent 0 "/Game/CommunityPlant/Assets/HouseAssets/Materials/Hallway_Materials/M_H_SunSetOverlayBlend_Inst.M_H_SunSetOverlayBlend_Inst"))
    (:`2`
      (`PaperTileMapComponent.SetTileMap` _rendercomponent "/Game/CommunityPlant/Assets/HouseAssets/TileMaps/HallwayTilemaps/N_HallwaySpriteSheet_TileMap.N_HallwaySpriteSheet_TileMap")
      (`PrimitiveComponent.SetMaterial` _rendercomponent 0 "/Game/CommunityPlant/Assets/HouseAssets/Materials/Hallway_Materials/M_HI_NightOverlayInstance.M_HI_NightOverlayInstance"))))

(fn `FindNum`
  (returns (DayOut :type Integer))
  (bind _daynum (`self.DayNum`))
  (if (< _daynum 2)
    (bind _result (`/Engine/EditorBlueprintResources/StandardMacros.IncrementInt` _daynum)
      (:`  `
        (return _result)))
    (else
      (bind _output_get (set `self.DayNum` 0))
      (return _output_get))))

(fn `UserConstructionScript`)